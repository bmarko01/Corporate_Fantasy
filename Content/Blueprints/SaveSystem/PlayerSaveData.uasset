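; PlayerSaveData is a save game object that stores the player's level, current objective, last save point and level name.
; SavePlayerData copies level and objective from the player character and writes the object to its slot.
; LoadPlayerData copies those two values back onto the character without reading from disk.
; SavePoint calls SavePlayerData, records the point's player start tag and the level name, then writes the slot again.
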(event Custom|SavePlayerData
  (params (PlayerCharacter :type Main%20Character%20BP%20Object%20Reference))
  (Variables|Default|SetPlayerLevel (Variables|/Game/Blueprints/MainCharacter/MainCharacter_BP.MainCharacter_BP_C|GetPlayerLevel PlayerCharacter))
  (Variables|Default|SetCurrent%20Objective (Variables|/Game/Blueprints/MainCharacter/MainCharacter_BP.MainCharacter_BP_C|GetCurrentObjective PlayerCharacter))
  (SaveGame|SaveGametoSlot self (Variables|Default|GetSlot%20Name)))

(event Custom|LoadPlayerData
  (params (PlayerCharacter :type Main%20Character%20BP%20Object%20Reference))
  (Variables|/Game/Blueprints/MainCharacter/MainCharacter_BP.MainCharacter_BP_C|SetPlayerLevel PlayerCharacter (Variables|Default|GetPlayerLevel))
  (Variables|/Game/Blueprints/MainCharacter/MainCharacter_BP.MainCharacter_BP_C|SetCurrentObjective PlayerCharacter (Variables|Default|GetCurrent%20Objective)))

(event Custom|SavePoint
  (params (SavePoint :type Save%20Point%20Object%20Reference) (Player :type Main%20Character%20BP%20Object%20Reference) (LevelName :type Name))
  (CallFunction|SavePlayerData Player)
  (Variables|Default|SetSavePointName (Utilities|String|ToString(Name) (Variables|/Script/Engine.PlayerStart|GetPlayerStartTag SavePoint)))
  (Variables|Default|SetLevelName LevelName)
  (SaveGame|SaveGametoSlot self (Variables|Default|GetSlot%20Name)))