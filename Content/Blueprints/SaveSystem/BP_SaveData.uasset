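; BP_SaveData is the save data container that holds player progress, per-level state and the last level.
; StorePlayerData copies objectives, health, experience, level and perk points from the player, plus inventory and skill unlocks from its components.
; StoreLevelData writes the player's location into a map keyed by level name, keeping one entry per level.
; StoreGameData records the last level; the functions shown only capture values, with no disk write or restore.
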(fn StorePlayerData
  (params (Player :type Main%20Character%20BP%20Object%20Reference))
  (Variables|PlayerData|SetObjectives (Variables|/Game/Blueprints/MainCharacter/MainCharacter_BP.MainCharacter_BP_C|GetObjectives Player))
  (Variables|PlayerData|SetPlayerHealth (Variables|/Game/Blueprints/MainCharacter/MainCharacter_BP.MainCharacter_BP_C|GetHealth Player))
  (Variables|PlayerData|SetPlayerHealthMax (Variables|/Game/Blueprints/MainCharacter/MainCharacter_BP.MainCharacter_BP_C|GetHealthMax Player))
  (Variables|PlayerData|SetExperiencePoints (Variables|/Game/Blueprints/MainCharacter/MainCharacter_BP.MainCharacter_BP_C|GetExperiencePoints Player))
  (Variables|PlayerData|SetPlayerLevel (Variables|/Game/Blueprints/MainCharacter/MainCharacter_BP.MainCharacter_BP_C|GetPlayerLevel Player))
  (Variables|PlayerData|SetInventory (Variables|/Game/Blueprints/InventorySystem/InventoryComponent.InventoryComponent_C|GetInventory (Variables|/Game/Blueprints/MainCharacter/MainCharacter_BP.MainCharacter_BP_C|GetInventoryComponent Player)))
  (Variables|PlayerData|SetSkillUnlocks (Variables|/Game/Blueprints/Skill_System/Skill_System_Component.Skill_System_Component_C|GetSkillUnlocks (Variables|/Game/Blueprints/MainCharacter/MainCharacter_BP.MainCharacter_BP_C|GetSkill_System_Component Player)))
  (Variables|PlayerData|SetPerkPoints (Variables|/Game/Blueprints/MainCharacter/MainCharacter_BP.MainCharacter_BP_C|GetPerkPoints Player)))

(fn StoreLevelData
  (params (LevelName :type String) (Player :type Main%20Character%20BP%20Object%20Reference))
  (Utilities|Map|Add (Variables|LevelData|GetLevelData) LevelName (Utilities|Struct|MakeELevelSaveData (Transformation|GetActorLocation Player))))

(fn StoreGameData
  (params (LastLevel :type String))
  (Variables|GameData|SetLastLevel LastLevel))