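; Base NPC pawn that players can talk to and that either roams or walks to a target actor.
; On begin play it passes its DialogueTree to its NPC_AI controller unless RandomDialogue is set, and Interact has that controller start dialogue.
; Tick applies walk speed, then issues AI moves to random reachable nearby points after random delays, or toward TargetActor, tracking IsMoving.
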(event EventTick
  (params (DeltaSeconds :type Float%20%28single-precision%29))
  (Variables|/Script/Engine.CharacterMovementComponent|SetMaxWalkSpeed (Variables|Character|GetCharacterMovement) (Variables|Default|GetMax%20Walk%20Speed))
  (if (Variables|Default|GetRoaming?)
    (Utilities|FlowControl|Delay (Math|Random|RandomFloatinRange 1.0 3.0))
    (Variables|Default|SetIsMoving? true)
    (AI|AIMoveTo self (.RandomLocation (AI|Navigation|GetRandomReachablePointinRadius (Transformation|GetActorLocation) (Variables|Default|GetMoveToRadius) 0 0)) 0 5.0 false
      (:OnSuccess
        _)
      (:OnFail
        _))
    (Variables|Default|SetIsMoving? false)
    (else
      (Variables|Default|SetIsMoving? true)
      (AI|AIMoveTo self "0, 0, 0" (Variables|Default|GetTarget%20Actor) 2e+01 false
        (:OnSuccess
          _)
        (:OnFail
          _))
      (Variables|Default|SetIsMoving? false))))

(event EventInteract
  (params (Interactor :type Actor%20Object%20Reference))
  (bind _asnpc_ai (Utilities|Casting|CastToNPC_AI (AI|GetAIController self)))
  (Default|StartDialogue _asnpc_ai))

(event EventBeginPlay
  (bind _asnpc_ai (Utilities|Casting|CastToNPC_AI (AI|GetAIController self)))
  (if (not (Variables|Default|GetRandom%20Dialogue?))
    (Variables|/Game/Blueprints/NPCs/NPC_AI.NPC_AI_C|SetDialogueTree _asnpc_ai (Variables|Default|GetDialogueTree))))

(fn ConstructionScript)