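; Level generator actor that builds a randomized NumX by NumY grid of streamed level tiles centered on itself at BeginPlay.
; Each cell spawns a random streaming level instance from the default LvlNames, rotated in random 90-degree yaw steps and block-loaded.
; SpecificLvlInfo entries override the pool at matching 1-based coordinates, which can be randomized first, with the first match winning.
; An unconnected snippet would move player controller 0 to a PlayerStart.
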(event EventBeginPlay
  (CallFunction|CheckforEntriesThatNeedCoordinates)
  (for _index (range 0 (- (Variables|Default|GetNumX) 1))
    (Variables|Default|SetLoopX _index)
    (for _index_2 (range 0 (- (Variables|Default|GetNumY) 1))
      (Variables|Default|SetLoopY _index_2)
      (bind (_lvldetails1 _foundinformation1) (CallFunction|CheckforSpecificLvlInfo))
      (if _foundinformation1
        (CallFunction|PickandSpawnLevelfromArray (.LvlNames (Utilities|Struct|BreakSpecificLvlInfo _lvldetails1)))
        (else
          (CallFunction|PickandSpawnLevelfromArray (Variables|Default|GetLvlNames)))))))

(fn ConstructionScript)

(fn PickandSpawnLevelfromArray
  (params (Lvl%20Names :type Array%20of%20Names))
  (bind _returnvalue (Class|LevelStreaming|CreateInstance (Class|GameplayStatics|GetStreamingLevel (Utilities|Array|Get(acopy) Lvl%20Names (Math|Random|RandomIntegerinRange 0 (Utilities|Array|LastIndex Lvl%20Names)))) (Utilities|String|Append (Utilities|String|ToString(Integer) (Variables|Default|GetLoopX)) "x" (Utilities|String|ToString(Integer) (Variables|Default|GetLoopY)) (Utilities|GetDisplayName self))))
  (Variables|/Script/Engine.LevelStreaming|SetLevelTransform _returnvalue (Math|Transform|MakeTransform (+ (Math|Vector|MakeVector (+ (- (* (Variables|Default|GetLoopX) (Variables|Default|GetLvlSize)) (/ (* (Variables|Default|GetNumX) (Variables|Default|GetLvlSize)) 2.0)) (/ (Variables|Default|GetLvlSize) 2.0)) (+ (- (* (Variables|Default|GetLoopY) (Variables|Default|GetLvlSize)) (/ (* (Variables|Default|GetNumY) (Variables|Default|GetLvlSize)) 2.0)) (/ (Variables|Default|GetLvlSize) 2.0)) 0.0) (Transformation|GetActorLocation)) (Math|Rotator|MakeRotator 0.0 0.0 (* (Math|Random|RandomIntegerinRange 0 3) 9e+01))))
  (Variables|/Script/Engine.LevelStreaming|SetbShouldBeLoaded _returnvalue true)
  (Variables|/Script/Engine.LevelStreaming|SetbShouldBeVisible _returnvalue true)
  (Variables|/Script/Engine.LevelStreaming|SetbShouldBlockOnLoad _returnvalue true))

(fn CheckforSpecificLvlInfo
  (LocalVariables|SetFoundInformation false)
  (for _array_element (Variables|Default|GetSpecificLvlInfo)
    (if (not (LocalVariables|GetFoundInformation))
      (if (and (== (+ (Math|Float|Round (.X (Math|Vector|BreakVector (.Coordinates (Utilities|Struct|BreakSpecificLvlInfo _array_element))))) -1) (Variables|Default|GetLoopX)) (== (+ (Math|Float|Round (.Y (Math|Vector|BreakVector (.Coordinates (Utilities|Struct|BreakSpecificLvlInfo _array_element))))) -1) (Variables|Default|GetLoopY)))
        (LocalVariables|SetLvlDetails _array_element)
        (LocalVariables|SetFoundInformation true))))
  (return (LocalVariables|GetLvlDetails) (LocalVariables|GetFoundInformation)))

(fn CheckforEntriesThatNeedCoordinates
  (for (_array_element _array_index) (Variables|Default|GetSpecificLvlInfo)
    (if (.GetRandomCoordinatesonBeginPlay? (Utilities|Struct|BreakSpecificLvlInfo _array_element))
      (Utilities|Array|SetArrayElem (Variables|Default|GetSpecificLvlInfo) _array_index (Utilities|Struct|MakeSpecificLvlInfo (Math|Vector|MakeVector (Math|Conversions|ToFloat(Integer) (Math|Random|RandomIntegerinRange 1 (Variables|Default|GetNumX))) (Math|Conversions|ToFloat(Integer) (Math|Random|RandomIntegerinRange 1 (Variables|Default|GetNumY))) 0.0) (.LvlNames (Utilities|Struct|BreakSpecificLvlInfo _array_element)) (.GetRandomCoordinatesonBeginPlay? (Utilities|Struct|BreakSpecificLvlInfo _array_element))))))
  (return))