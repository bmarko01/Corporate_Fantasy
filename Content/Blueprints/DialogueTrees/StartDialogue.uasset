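; StartDialogue is a behavior tree task that opens a dialogue with the controlled NPC.
; Unless the completed blackboard flag is set, it puts the NPC's name on the HUD dialogue box, shows it and stores that widget in the blackboard.
; It also disables player input and shows the mouse cursor, then finishes successfully.
; If the flag is set or a cast fails, the task never calls FinishExecute.
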(event EventReceiveExecuteAI
  (params (OwnerController :type AI%20Controller%20Object%20Reference) (ControlledPawn :type Pawn%20Object%20Reference))
  (bind _returnvalue (Game|GetPlayerController 0))
  (bind _asnpc_base (Utilities|Casting|CastToNPC_base ControlledPawn))
  (Variables|Default|SetNPCPawn _asnpc_base)
  (if (not (Class|BTFunctionLibrary|GetBlackboardValueasBool (Variables|Default|GetBB_Completed)))
    (bind _asmain_gamemode (Utilities|Casting|CastToMainGamemode (Game|GetGameMode)))
    (Variables|/Game/Blueprints/UI/DialogueBox.DialogueBox_C|SetSpeakerName (Variables|/Game/Blueprints/UI/HeadsUpDisplay.HeadsUpDisplay_C|GetDialogueBox (Variables|/Game/Blueprints/GameSettings/MainGamemode.MainGamemode_C|GetHeadsUpDisplay _asmain_gamemode)) (Variables|/Game/Blueprints/NPCs/NPC_base.NPC_base_C|GetName (Variables|Default|GetNPCPawn)))
    (Widget|SetVisibility (Variables|/Game/Blueprints/UI/HeadsUpDisplay.HeadsUpDisplay_C|GetDialogueBox (Variables|/Game/Blueprints/GameSettings/MainGamemode.MainGamemode_C|GetHeadsUpDisplay _asmain_gamemode)) "Visible")
    (Class|BTFunctionLibrary|SetBlackboardValueasObject (Variables|Default|GetBB_DialogueUI) (Variables|/Game/Blueprints/UI/HeadsUpDisplay.HeadsUpDisplay_C|GetDialogueBox (Variables|/Game/Blueprints/GameSettings/MainGamemode.MainGamemode_C|GetHeadsUpDisplay _asmain_gamemode)))
    (Input|DisableInput (Game|GetPlayerCharacter 0) _returnvalue)
    (Variables|/Script/Engine.PlayerController|SetbShowMouseCursor _returnvalue true)
    (AI|BehaviorTree|FinishExecute true)))