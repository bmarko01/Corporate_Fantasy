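; Behavior tree task for dialogue trees that shows a question with selectable responses and waits for a choice.
; It gets the DialogueBox widget from the blackboard, sets its text, and adds a response list containing one clickable widget per response.
; Each widget's click event is bound to a callback, so the choice is written to the blackboard as a string, the list is removed, and the task finishes successfully.
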(event Custom|ResponseReceived
  (params (ResponseReceived :type Text))
  (Class|BTFunctionLibrary|SetBlackboardValueasString (Variables|Default|GetBB_Response) (Utilities|String|ToString(Text) ResponseReceived))
  (Widget|RemovefromParent (Variables|Default|GetResponseListUI))
  (AI|BehaviorTree|FinishExecute true))

(event EventReceiveExecuteAI
  (params (OwnerController :type AI%20Controller%20Object%20Reference) (ControlledPawn :type Pawn%20Object%20Reference))
  (bind _asdialogue_box (Utilities|Casting|CastToDialogueBox (Class|BTFunctionLibrary|GetBlackboardValueasObject (Variables|Default|GetBB_DialogueUI))))
  (bind _output_get (Variables|Default|SetDialogue%20Box%20UI _asdialogue_box))
  (Variables|/Game/Blueprints/UI/DialogueBox.DialogueBox_C|SetDialogueText _output_get (Variables|Default|GetQuestion))
  (CallFunction|PrepareResponses))

(fn PrepareResponses
  (bind _returnvalue (UserInterface|CreateWidget "/Game/Blueprints/UI/ResponseListUI.ResponseListUI_C"))
  (bind _output_get (Variables|Default|SetResponseListUI _returnvalue))
  (Class|Overlay|AddChildtoOverlay (Variables|/Game/Blueprints/UI/DialogueBox.DialogueBox_C|GetResponseListPanel (Variables|Default|GetDialogue%20Box%20UI)) _output_get)
  (for _array_element (Variables|Default|GetResponses)
    (bind _returnvalue_2 (UserInterface|CreateWidget "/Game/Blueprints/UI/ResponseUI.ResponseUI_C" 0 _array_element))
    (Class|VerticalBox|AddChildtoVerticalBox (Variables|/Game/Blueprints/UI/ResponseListUI.ResponseListUI_C|GetResponseList (Variables|Default|GetResponseListUI)) _returnvalue_2)
    (EventDispatchers|BindEventtoResponseClicked _returnvalue_2 (EventDispatchers|CreateEvent :!event Custom|ResponseReceived))))