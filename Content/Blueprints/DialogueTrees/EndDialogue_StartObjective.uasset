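; Behavior tree task that closes an NPC dialogue and gives the player a new objective.
; It hides the blackboard's dialogue widget, tells the NPC AI controller to end dialogue, and restores game-only input to the player.
; If the main character can accept an objective, it assigns one, clears that flag, calls SlideOn and plays a sound.
; The task finishes only on that accepting branch.
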(event EventReceiveExecuteAI
  (params (OwnerController :type AI%20Controller%20Object%20Reference) (ControlledPawn :type Pawn%20Object%20Reference))
  (bind _returnvalue (Game|GetPlayerController 0))
  (bind _returnvalue_2 (Game|GetPlayerCharacter 0))
  (bind _aswidget (Utilities|Casting|CastToWidget (Class|BTFunctionLibrary|GetBlackboardValueasObject (Variables|Default|GetBB_DialogueUI))))
  (Widget|SetVisibility _aswidget "Hidden")
  (bind _asnpc_ai (Utilities|Casting|CastToNPC_AI OwnerController))
  (Default|EndDialogue _asnpc_ai)
  (Variables|/Script/Engine.PlayerController|SetbShowMouseCursor _returnvalue false)
  (Input|SetInputModeGameOnly _returnvalue)
  (Input|EnableInput _returnvalue_2 _returnvalue)
  (bind _asmain_character_bp (Utilities|Casting|CastToMainCharacter_BP _returnvalue_2))
  (if (Variables|/Game/Blueprints/MainCharacter/MainCharacter_BP.MainCharacter_BP_C|GetCan%20Accept%20Objective _asmain_character_bp)
    (Variables|/Game/Blueprints/MainCharacter/MainCharacter_BP.MainCharacter_BP_C|SetCurrentObjective _asmain_character_bp (Variables|Default|GetObjective))
    (Variables|/Game/Blueprints/MainCharacter/MainCharacter_BP.MainCharacter_BP_C|SetCan%20Accept%20Objective _asmain_character_bp false)
    (Default|Slideon _asmain_character_bp)
    (Audio|PlaySound2D 0 1.0 1.0 0.0 0 0)
    (AI|BehaviorTree|FinishExecute true)))