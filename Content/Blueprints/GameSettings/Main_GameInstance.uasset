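; Game instance that manages save data: a global game save plus per-slot player saves.
; On Init it loads the "GameSaveData" slot, or creates a new save object in memory if none exists.
; LoadSaveGame loads the named slot as the current player save, or creates it, registers its name in the global slot list and writes both saves to disk.
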(event Custom|LoadSaveGame
  (params (SaveSlotName :type String))
  (bind _returnvalue (SaveGame|DoesSaveGameExist SaveSlotName))
  (if _returnvalue
    (bind _returnvalue_2 (SaveGame|LoadGamefromSlot SaveSlotName))
    (bind _asplayer_save_data (Utilities|Casting|CastToPlayerSaveData _returnvalue_2))
    (bind _output_get (Variables|Default|SetCurrentSaveData _asplayer_save_data))
    (Variables|/Game/Blueprints/SaveSystem/PlayerSaveData.PlayerSaveData_C|SetSlot%20Name _output_get SaveSlotName)
    (else
      (bind _returnvalue_3 (SaveGame|CreateSaveGameObject "/Game/Blueprints/SaveSystem/PlayerSaveData.PlayerSaveData_C"))
      (bind _output_get_2 (Variables|Default|SetCurrentSaveData _returnvalue_3))
      (bind _output_get_3 (Variables|/Game/Blueprints/SaveSystem/PlayerSaveData.PlayerSaveData_C|SetSlot%20Name _output_get_2 SaveSlotName))
      (Utilities|Array|Add (Variables|/Game/Blueprints/SaveSystem/GameSaveData.GameSaveData_C|GetSaveSlots (Variables|Default|GetAs%20Game%20Save%20Data)) _output_get_3)
      (SaveGame|SaveGametoSlot (Variables|Default|GetAs%20Game%20Save%20Data) "GameSaveData")
      (SaveGame|SaveGametoSlot (Variables|Default|GetCurrentSaveData) SaveSlotName))))

(event EventInit
  (bind _returnvalue (SaveGame|DoesSaveGameExist "GameSaveData"))
  (if _returnvalue
    (bind _returnvalue_2 (SaveGame|LoadGamefromSlot "GameSaveData"))
    (bind _asgame_save_data (Utilities|Casting|CastToGameSaveData _returnvalue_2))
    (Variables|Default|SetAs%20Game%20Save%20Data _asgame_save_data)
    (else
      (bind _returnvalue_3 (SaveGame|CreateSaveGameObject "/Game/Blueprints/SaveSystem/GameSaveData.GameSaveData_C"))
      (Variables|Default|SetAs%20Game%20Save%20Data _returnvalue_3))))