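; MainGamemode is the game mode that spawns new players, sets up the HUD and starts a save data check.
; Each new player restarts at the player start found by the name taken from the options string minus its first character.
; On BeginPlay it creates the HUD widget and hands it to the main character.
; It then has the game instance run CheckValidSaveDataEnv.
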(event EventHandleStartingNewPlayer
  (params (NewPlayer :type Player%20Controller%20Object%20Reference))
  (bind _optionsstring (Variables|Default|GetOptionsString))
  (Class|GameModeBase|RestartPlayeratPlayerStart NewPlayer (Class|GameModeBase|FindPlayerStart NewPlayer (Utilities|String|GetSubstring _optionsstring 1 (- (Utilities|String|Len _optionsstring) 1)))))

(event EventBeginPlay
  (Utilities|FlowControl|Sequence
    (:then_0
      (bind _returnvalue (UserInterface|CreateWidget "/Game/Blueprints/UI/HeadsUpDisplay.HeadsUpDisplay_C"))
      (bind _output_get (Variables|Default|SetHeadsUpDisplay _returnvalue))
      (UserInterface|Viewport|AddtoViewport _output_get 0)
      (Variables|/Game/Blueprints/MainCharacter/MainCharacter_BP.MainCharacter_BP_C|SetPlayerHUD (CallFunction|GetMainCharacter) _output_get))
    (:then_1
      (Default|CheckValidSaveDataEnv (CallFunction|GetMainGameInstance)))))

(fn ConstructionScript)