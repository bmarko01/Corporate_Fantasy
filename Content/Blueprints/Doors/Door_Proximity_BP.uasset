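; Proximity sliding door that opens only for a main character with the "steel_grip" skill at tier 2 or higher.
; Box overlap queries the character's SkillSystemComponent, then plays the DoorAnimation timeline, which sets the door mesh's relative location.
; Leaving the box reverses the timeline if the skill query succeeds, without checking the tier.
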(event OnComponentBeginOverlap(Box)
  (params (OverlappedComponent :type Primitive%20Component%20Object%20Reference) (OtherActor :type Actor%20Object%20Reference) (OtherComp :type Primitive%20Component%20Object%20Reference) (OtherBodyIndex :type Integer) (bFromSweep :type Boolean) (SweepResult :type Hit%20Result%20Structure%20%28by%20ref%29))
  (bind _asmain_character_bp (Utilities|Casting|CastToMainCharacter_BP OtherActor))
  (bind (_success _tierlevel) (Default|QuerySkill (Variables|/Game/Blueprints/MainCharacter/MainCharacter_BP.MainCharacter_BP_C|GetSkill_System_Component _asmain_character_bp) "steel_grip"))
  (if (and _success (>= _tierlevel 2))
    (bind _doorsliding (Timeline|DoorAnimation Play)
      (:Update
        (Transformation|SetRelativeLocation (Variables|Default|GetDoorMesh) _doorsliding false false)))))

(event OnComponentEndOverlap(Box)
  (params (OverlappedComponent :type Primitive%20Component%20Object%20Reference) (OtherActor :type Actor%20Object%20Reference) (OtherComp :type Primitive%20Component%20Object%20Reference) (OtherBodyIndex :type Integer))
  (bind _asmain_character_bp (Utilities|Casting|CastToMainCharacter_BP OtherActor))
  (bind _success (Default|QuerySkill (Variables|/Game/Blueprints/MainCharacter/MainCharacter_BP.MainCharacter_BP_C|GetSkill_System_Component _asmain_character_bp) "steel_grip"))
  (if _success
    (bind _doorsliding (Timeline|DoorAnimation Reverse)
      (:Update
        (Transformation|SetRelativeLocation (Variables|Default|GetDoorMesh) _doorsliding false false)))))

(fn ConstructionScript)