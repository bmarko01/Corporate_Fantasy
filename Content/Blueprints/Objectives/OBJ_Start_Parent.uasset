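; Parent pickup actor that starts an objective when the player interacts with it.
; Interact adds its item to the interactor's inventory component, then asks the main character to add its objective.
; On success it triggers the character's SlideOn, plays a 2D sound and destroys itself.
; UseItem always returns false.
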(event EventInteract
  (params (Interactor :type Actor%20Object%20Reference))
  (bind _success (Default|AddtoInventory (Actor|GetComponentbyClass Interactor "/Game/Blueprints/InventorySystem/InventoryComponent.InventoryComponent_C") (Utilities|Struct|MakeSlotStructure (Variables|Default|GetItemStructure) 1)))
  (if _success
    (bind _asmain_character_bp (Utilities|Casting|CastToMainCharacter_BP (Game|GetPlayerCharacter 0)))
    (bind _success_2 (Default|TryAddObjective _asmain_character_bp (Variables|Default|GetObjective)))
    (if _success_2
      (Default|Slideon _asmain_character_bp)
      (Audio|PlaySound2D 0 1.0 1.0 0.0 0 0)
      (Actor|DestroyActor))))

(fn ConstructionScript)

(fn UseItem
  (return false))