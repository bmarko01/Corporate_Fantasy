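; Skill system component that records which skills are unlocked and at what tier level.
; The SkillUnlocks map stores a tier per row name; AddSkill inserts a skill at tier 1 or increments its existing tier, always returning true with no upper limit check.
; QuerySkill looks up a row name and returns whether it is unlocked along with its tier, or zero when absent.
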(event EventBeginPlay)

(event EventTick
  (params (DeltaSeconds :type Float%20%28single-precision%29)))

(fn AddSkill
  (params (row_name :type String))
  (bind _skillunlocks (Variables|Default|GetSkillUnlocks))
  (bind (_value _returnvalue) (Utilities|Map|Find _skillunlocks row_name))
  (if _returnvalue
    (Utilities|Map|Add (Variables|Default|GetSkillUnlocks) row_name (+ _value 1))
    (return true)
    (else
      (Utilities|Map|Add (Variables|Default|GetSkillUnlocks) row_name 1)
      (return true))))

(fn QuerySkill
  (params (RowName :type String))
  (bind _skillunlocks (Variables|Default|GetSkillUnlocks))
  (bind (_value _returnvalue) (Utilities|Map|Find _skillunlocks RowName))
  (if _returnvalue
    (return true _value)
    (else
      (return false 0))))